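; MasterTile is a track tile for an endless runner that spawns its own pickups and obstacles on BeginPlay.
; SpawnObs makes a random roll to place a pickup, block or pipe at Left, Middle or Right, with Right filled only alongside a middle block.
; When the character overlaps Box, the tile has the game mode spawn another tile, adds multiplied points, raises walk speed within limits, then destroys itself after a delay.
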(event `self.ReceiveBeginPlay`
  (`self.SpawnObs`))

(event `self.Box.OnComponentBeginOverlap`
  (params (OverlappedComponent :type "PrimitiveComponent Object Reference") (OtherActor :type "Actor Object Reference") (OtherComp :type "PrimitiveComponent Object Reference") (OtherBodyIndex :type Integer) (bFromSweep :type Boolean) (SweepResult :type "HitResult Structure (by ref)"))
  (cast `/Game/ThirdPersonBP/Blueprints/ThirdPersonCharacter` OtherActor)
  (bind _asthird_person_game_mode (cast `/Game/ThirdPersonBP/Blueprints/ThirdPersonGameMode` (`GameplayStatics.GetGameMode`)))
  (`/Game/ThirdPersonBP/Blueprints/ThirdPersonGameMode.Spawn Tile` _asthird_person_game_mode)
  (bind _asthird_person_game_mode_2 (cast `/Game/ThirdPersonBP/Blueprints/ThirdPersonGameMode` (`GameplayStatics.GetGameMode`)))
  (set `/Game/ThirdPersonBP/Blueprints/ThirdPersonGameMode.Current Points` (+ (* 1 (`/Game/ThirdPersonBP/Blueprints/ThirdPersonGameMode.Points Multiplier` _asthird_person_game_mode_2)) (`/Game/ThirdPersonBP/Blueprints/ThirdPersonGameMode.Current Points` _asthird_person_game_mode_2)) _asthird_person_game_mode_2)
  (bind _asthird_person_character (cast `/Game/ThirdPersonBP/Blueprints/ThirdPersonCharacter` (`GameplayStatics.GetPlayerCharacter` 0)))
  (bind _charactermovement (`Character.CharacterMovement` _asthird_person_character))
  (set `CharacterMovementComponent.MaxWalkSpeed` (`KismetMathLibrary.FClamp` (* (`CharacterMovementComponent.MaxWalkSpeed` _charactermovement) 1.04) 600.0 2600.0) _charactermovement)
  (`KismetSystemLibrary.Delay` 3.0)
  (`self.K2_DestroyActor`))

(fn `SpawnObs`
  (bind _returnvalue (`SceneComponent.K2_GetComponentToWorld` (`self.Right`)))
  (bind _returnvalue_2 (`SceneComponent.K2_GetComponentToWorld` (`self.Left`)))
  (bind _returnvalue_3 (`SceneComponent.K2_GetComponentToWorld` (`self.Middle`)))
  ;[1 1 1] Lane 0
  (switch `int` (`KismetMathLibrary.RandomIntegerInRange` 0 4)
    (:`0`
      (`|SpawnActorFromClass` "/Game/RunALotFIles/Blueprints/pickup.pickup_C" _returnvalue_2 "Undefined" "OverrideRootScale" null null))
    (:`1`
      (`|SpawnActorFromClass` "/Game/RunALotFIles/Blueprints/block_obsticle1.block_obsticle1_C" _returnvalue_2 "Undefined" "OverrideRootScale" null null))
    (:`2`
      (`|SpawnActorFromClass` "/Game/RunALotFIles/Blueprints/pipe_obsticle.pipe_obsticle_C" _returnvalue_2 "Undefined" "OverrideRootScale" null null))
    (:`3`
      ;[1 1 1] Lane1
      (`|SpawnActorFromClass` "/Game/RunALotFIles/Blueprints/block_obsticle1.block_obsticle1_C" _returnvalue_3 "Undefined" "OverrideRootScale" null null)
      ;[1 1 1] Lane2
      (switch `int` (`KismetMathLibrary.RandomIntegerInRange` 0 2)
        (:`0`
          (`|SpawnActorFromClass` "/Game/RunALotFIles/Blueprints/pickup.pickup_C" _returnvalue "Undefined" "OverrideRootScale" null null))
        (:`1`
          (`|SpawnActorFromClass` "/Game/RunALotFIles/Blueprints/block_obsticle1.block_obsticle1_C" _returnvalue "Undefined" "OverrideRootScale" null null))
        (:`2`
          (`|SpawnActorFromClass` "/Game/RunALotFIles/Blueprints/pipe_obsticle.pipe_obsticle_C" _returnvalue "Undefined" "OverrideRootScale" null null))))
    (:`4`
      (`|SpawnActorFromClass` "/Game/RunALotFIles/Blueprints/pipe_obsticle.pipe_obsticle_C" _returnvalue_3 "Undefined" "OverrideRootScale" null null))))

(fn `UserConstructionScript`)